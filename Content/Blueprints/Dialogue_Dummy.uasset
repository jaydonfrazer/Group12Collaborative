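; Dialogue test actor that shows a conversation widget while the player character is inside its box trigger.
; Overlap swaps the cube's material and creates the DialogueUi widget; leaving restores the material and removes the widget.
; EventDialogueOccurs passes ConversationText to the widget, reveals it and advances TextRow, removing it at the last row.
; A DoOnce gates each advance and is reset immediately afterwards through ResetDialogue.
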(event `self.Box.OnComponentBeginOverlap`
  (params (OverlappedComponent :type "PrimitiveComponent Object Reference") (OtherActor :type "Actor Object Reference") (OtherComp :type "PrimitiveComponent Object Reference") (OtherBodyIndex :type Integer) (bFromSweep :type Boolean) (SweepResult :type "HitResult Structure (by ref)"))
  (cast `/Game/Blueprints/PlayerCharacter_BP` OtherActor)
  (`PrimitiveComponent.SetMaterial` (`self.Cube`) 0 "/Game/StarterContent/Materials/M_Ceramic_Tile_Checker.M_Ceramic_Tile_Checker")
  (bind _returnvalue (`|CreateWidget` "/Game/Blueprints/DialogueUi.DialogueUi_C"))
  (bind _output_get (set `self.DialogueUi` _returnvalue))
  (`UserWidget.AddToViewport` _output_get 0))

(event `self.Box.OnComponentEndOverlap`
  (params (OverlappedComponent :type "PrimitiveComponent Object Reference") (OtherActor :type "Actor Object Reference") (OtherComp :type "PrimitiveComponent Object Reference") (OtherBodyIndex :type Integer))
  (bind _dialogueui (`self.DialogueUi`))
  (cast `/Game/Blueprints/PlayerCharacter_BP` OtherActor)
  (`PrimitiveComponent.SetMaterial` (`self.Cube`) 0 "/Game/Model/Assets/initialShadingGroup.initialShadingGroup")
  (`/Engine/EditorBlueprintResources/StandardMacros.IsValid` _dialogueui
    (:`Is Valid`
      (`Widget.RemoveFromParent` _dialogueui))))

(event `/Game/Blueprints/DialogueInterface.EventDialogueOccurs`
  (bind _returnvalue (+ (`/Game/Blueprints/DialogueUi.TextRow` (`self.DialogueUi`)) 1))
  (`/Engine/EditorBlueprintResources/StandardMacros.DoOnce` false :!label _label
    (:`Completed`
      (set `/Game/Blueprints/DialogueUi.Text` (`self.ConversationText`) (`self.DialogueUi`))
      (`Widget.SetVisibility` (`/Game/Blueprints/DialogueUi.BoxImage` (`self.DialogueUi`)) "Visible")
      (`Widget.SetVisibility` (`/Game/Blueprints/DialogueUi.TextBlock_88` (`self.DialogueUi`)) "Visible")
      (if (> _returnvalue (- (`KismetArrayLibrary.Array_Length` (`self.ConversationText`)) 1))
        (`Widget.RemoveFromParent` (`self.DialogueUi`))
        (`self.ResetDialogue`)
        (else
          (set `/Game/Blueprints/DialogueUi.TextRow` _returnvalue (`self.DialogueUi`))
          (`self.ResetDialogue`))))))

(event `ResetDialogue`
  (goto _label :!via `Reset`))

(fn `UserConstructionScript`)