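; BP_HomingMissile_TS is a homing projectile in the test bed boss content that damages the player on overlap.
; A short timer started on BeginPlay turns on ProjectileMovement homing and targets the root component of player character 0, so tracking begins just after spawn.
; An overlap with a PlayerCharacter applies the Damage value and destroys the missile, while other actors are ignored.
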(event `self.ReceiveBeginPlay`
  (`KismetSystemLibrary.K2_SetTimerDelegate` (delegate `StartHoming`) 0.2))

(event `StartHoming`
  (bind _projectilemovement (`self.ProjectileMovement`))
  (set `ProjectileMovementComponent.bIsHomingProjectile` true _projectilemovement)
  (set `ProjectileMovementComponent.HomingTargetComponent` (`Actor.RootComponent` (`GameplayStatics.GetPlayerCharacter` 0)) _projectilemovement))

(event `self.ReceiveActorBeginOverlap`
  (params (OtherActor :type "Actor Object Reference"))
  (bind _asplayer_character (cast `PlayerCharacter` OtherActor))
  (`GameplayStatics.ApplyDamage` _asplayer_character (`self.Damage`))
  (`self.K2_DestroyActor`))

(fn `UserConstructionScript`)