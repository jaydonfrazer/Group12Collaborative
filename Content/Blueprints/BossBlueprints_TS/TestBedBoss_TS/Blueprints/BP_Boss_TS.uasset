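; 2D flipbook boss that patrols four interpolated control points while attacking the player.
; Brain, started at BeginPlay, loops a delay-timed pattern of timed sweeps, shotgun bursts, fan shots and homing missiles, aimed in the XZ plane.
; Tick sets DamagePhase below a health threshold and handles death with an explosion.
; DamagePhase selects the attack pattern and patrol speed only at BeginPlay and construction, so later changes affect only flipbook branches.
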(event `Brain`
  ;[1 1 1] Main Sequence
  (if (> (`self.Health`) 0.0)
    (if (`self.DamagePhase`)
      (if true :!label _label
        (`KismetSystemLibrary.Delay` 5.0)
        (`|ExecutionSequence`
          (:`then_0`
            (`self.FiringAnim`)
            (`self.DelaySpreadShot` 200.0 20 0.02
              (:`Finished`
                (`self.EndFiringAnim`)
                (`KismetSystemLibrary.Delay` 1.0)
                (`self.FireMissile`)
                (`KismetSystemLibrary.Delay` 1.0)
                (`self.FiringAnim`)
                (`self.DelaySpreadShot` 200.0 25 0.02
                  (:`Finished`
                    (`self.EndFiringAnim`)
                    (`KismetSystemLibrary.Delay` 3.0)
                    (`self.Shotgun` 8 30.0)
                    (`KismetSystemLibrary.Delay` 3.0)
                    (`self.Shotgun` 8 30.0)
                    (`KismetSystemLibrary.Delay` 3.0)
                    (`self.FireMissile`))))))
          (:`then_1`
            (goto _label))))
      (else
        (if true :!label _label_2
          (`KismetSystemLibrary.Delay` 5.0)
          (`|ExecutionSequence`
            (:`then_0`
              (`self.FiringAnim`)
              (`self.DelaySpreadShot` 360.0 10 0.05
                (:`Finished`
                  (`self.EndFiringAnim`)
                  (`KismetSystemLibrary.Delay` 2.0)
                  (`self.FireMissile`)
                  (`KismetSystemLibrary.Delay` 2.0)
                  (`self.FiringAnim`)
                  (`self.DelaySpreadShot` 360.0 16 0.05
                    (:`Finished`
                      (`self.EndFiringAnim`)
                      (`KismetSystemLibrary.Delay` 3.0)
                      (`self.Shotgun` 5 25.0)
                      (`KismetSystemLibrary.Delay` 3.0)
                      (`self.Shotgun` 5 25.0)
                      (`KismetSystemLibrary.Delay` 3.0)
                      (`self.SpreadShot` 5 40.0))))))
            (:`then_1`
              (goto _label_2))))))))

(event `self.ReceiveBeginPlay`
  (`self.Brain`))

(event `self.ReceiveAnyDamage`
  (params (Damage :type "Float (single-precision)") (DamageType :type "DamageType Object Reference") (InstigatedBy :type "Controller Object Reference") (DamageCauser :type "Actor Object Reference"))
  ;[1 1 1] HandleDamage
  (set `self.Health` (- (`self.Health`) Damage))
  (`ActorComponent.Activate` (`self.Explosion`) true))

(event `StartFiring`
  (`self.FireMissile`))

(event `self.ReceiveTick`
  (params (DeltaSeconds :type "Float (single-precision)"))
  ;[1 1 1] Handle State
  (if (< (`self.Health`) 150.0)
    (if (<= (`self.Health`) 0.0)
      (`PaperFlipbookComponent.SetFlipbook` (`self.BossIdle_2`) null)
      (`ActorComponent.Activate` (`self.BigExplosion`) false)
      (`KismetSystemLibrary.Delay` 2.0)
      (`self.K2_DestroyActor`)
      (else
        (set `self.DamagePhase` true)
        (`PaperFlipbookComponent.SetFlipbook` (`self.BossIdle_2`) null)))
    (else
      (set `self.DamagePhase` false))))

(event `FiringAnim`
  (bind _bossidle_2 (`self.BossIdle_2`))
  ;[1 1 1] FlipbookHandles
  (if (`self.DamagePhase`)
    (`PaperFlipbookComponent.SetFlipbook` _bossidle_2 null)
    (else
      (`PaperFlipbookComponent.SetFlipbook` _bossidle_2 null))))

(event `EndFiringAnim`
  (bind _bossidle_2 (`self.BossIdle_2`))
  ;[1 1 1] FlipbookHandles
  (if (`self.DamagePhase`)
    (`PaperFlipbookComponent.SetFlipbook` _bossidle_2 null)
    (else
      (`PaperFlipbookComponent.SetFlipbook` _bossidle_2 null))))

(fn `Fire`
  (params (Rotation :type "Rotator Structure"))
  (`|SpawnActorFromClass` "/Script/Group12Project.BaseProjectile" (`KismetMathLibrary.MakeTransform` (`self.K2_GetActorLocation`) Rotation) "Undefined" "OverrideRootScale" null null)
  (`ActorComponent.Activate` (`self.Fireball`) true))

(fn `FireMissile`
  (`|SpawnActorFromClass` "/Game/Blueprints/BossBlueprints_TS/TestBedBoss_TS/Blueprints/BP_HomingMissile_TS.BP_HomingMissile_TS_C" (`KismetMathLibrary.MakeTransform` (`SceneComponent.K2_GetComponentLocation` (`self.MissileFirepoint`)) (struct :`Pitch` 90.0)) "Undefined" "OverrideRootScale" null null)
  (`ActorComponent.Activate` (`self.Missile`) false))

(fn `Shotgun`
  (params (NumberOfShots :type Integer) (Spread :type "Float (double-precision)"))
  (bind (_returnvalue_x _returnvalue_y _returnvalue_z) (`KismetMathLibrary.BreakVector` (`self.K2_GetActorLocation`)))
  (bind (_returnvalue_x_2 _returnvalue_y_2 _returnvalue_z_2) (`KismetMathLibrary.BreakVector` (`self.K2_GetActorLocation` (`GameplayStatics.GetPlayerCharacter` 0))))
  (for _ (range 1 (+ NumberOfShots 1))
    (`self.Fire` (`KismetMathLibrary.ComposeRotators` (`KismetMathLibrary.FindLookAtRotation` (`KismetMathLibrary.MakeVector` _returnvalue_x 0.0 _returnvalue_z) (`KismetMathLibrary.MakeVector` _returnvalue_x_2 0.0 _returnvalue_z_2)) (`KismetMathLibrary.MakeRotator` 0.0 (- (`KismetMathLibrary.RandomFloatInRange` 0.0 Spread) (/ Spread 2.0)))))))

(fn `SpreadShot`
  (params (NumberOfShots :type Integer) (Spread :type "Float (double-precision)"))
  (bind (_returnvalue_x _returnvalue_y _returnvalue_z) (`KismetMathLibrary.BreakVector` (`self.K2_GetActorLocation`)))
  (bind (_returnvalue_x_2 _returnvalue_y_2 _returnvalue_z_2) (`KismetMathLibrary.BreakVector` (`self.K2_GetActorLocation` (`GameplayStatics.GetPlayerCharacter` 0))))
  (for _index (range 1 (+ NumberOfShots 1))
    (`self.Fire` (`KismetMathLibrary.ComposeRotators` (`KismetMathLibrary.FindLookAtRotation` (`KismetMathLibrary.MakeVector` _returnvalue_x 0.0 _returnvalue_z) (`KismetMathLibrary.MakeVector` _returnvalue_x_2 0.0 _returnvalue_z_2)) (`KismetMathLibrary.MakeRotator` 0.0 (- (* _index (/ Spread (`KismetMathLibrary.Conv_IntToDouble` NumberOfShots))) (/ Spread 2.0)))))))

(fn `UserConstructionScript`
  (bind _interptomovement (`self.InterpToMovement`))
  ;[1 1 1] Movement
  (set `InterpToMovementComponent.ControlPoints` (`|MakeArray` (make `InterpControlPoint` (`self.PointA`)) (make `InterpControlPoint` (`self.PointB`)) (make `InterpControlPoint` (`self.PointC`)) (make `InterpControlPoint` (`self.PointD`))) _interptomovement)
  (if (`self.DamagePhase`)
    (set `InterpToMovementComponent.Duration` 3.0 _interptomovement)
    (else
      (set `InterpToMovementComponent.Duration` 10.0 _interptomovement))))