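; Player character Blueprint that handles pausing, game over and Paper2D sprite animation.
; The Pause input toggles game pause, input mode and a lazily created, cached pause menu widget.
; Tick polls Lives, creating and showing a new end screen every frame it equals zero, with the game set unpaused.
; Otherwise, Tick picks an idle, run-up or run-down flipbook from player speed and X velocity sign.
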(event `InputAction|Pause`
  (params (Key :type "Key Structure"))
  (bind _returnvalue (`GameplayStatics.GetPlayerController` 0))
  (bind _pausemenuref (`self.PauseMenuRef`))
  ;[1 1 1] Pause / Unpause Game
  (:`Pressed`
    (`/Engine/EditorBlueprintResources/StandardMacros.IsValid` (`self.PauseMenuRef`)
      (:`Is Valid`
        _)
      (:`Is Not Valid`
        (bind _returnvalue_2 (`|CreateWidget` "/Game/UI/PauseMenu_TS/PauseMenu_Widget_TS.PauseMenu_Widget_TS_C"))
        (set `self.PauseMenuRef` _returnvalue_2)))
    (if (`GameplayStatics.IsGamePaused`)
      (`Widget.RemoveFromParent` _pausemenuref)
      (`GameplayStatics.SetGamePaused` false)
      (`WidgetBlueprintLibrary.SetInputMode_GameOnly` _returnvalue)
      (else
        (`UserWidget.AddToViewport` _pausemenuref 0)
        (`GameplayStatics.SetGamePaused` true)
        (`WidgetBlueprintLibrary.SetInputMode_GameAndUIEx` _returnvalue _pausemenuref)))))

(event `self.ReceiveTick`
  (params (DeltaSeconds :type "Float (single-precision)"))
  (bind _playervelocity_x (`KismetMathLibrary.BreakVector` (`self.PlayerVelocity`)))
  ;[1 1 1] Event Tick
  ;;[1 1 1] Game Over
  (if (== (`self.Lives`) 0)
    (`GameplayStatics.SetGamePaused` false)
    (bind _returnvalue (`|CreateWidget` "/Game/UI/StartEndScreens_TS/EndScreen_Widget_TS.EndScreen_Widget_TS_C"))
    (`UserWidget.AddToViewport` _returnvalue 0)
    (else
      ;;[1 1 1] Sprite Manager
      (set `self.PlayerVelocity` (`self.GetVelocity` (`GameplayStatics.GetPlayerCharacter` 0)))
      (if (== (`KismetMathLibrary.VSize` (`self.PlayerVelocity`)) 0.0)
        (`PaperFlipbookComponent.SetFlipbook` (`self.PaperFlipbook`) "/Game/Material/Sprites/MC/2_Set/Idle/2_1_MC_Idle.2_1_MC_Idle")
        (else
          (`PaperFlipbookComponent.SetFlipbook` (`self.PaperFlipbook`) (select `bool` (< _playervelocity_x 0.0) :`false` "/Game/Material/Sprites/MC/2_Set/Run_Up/2_1_MC_Run_Up.2_1_MC_Run_Up" :`true` "/Game/Material/Sprites/MC/2_Set/Run_down/2_2_MC_Run_Down.2_2_MC_Run_Down" :!type "PaperFlipbook Object Reference")))))))

(fn `UserConstructionScript`)